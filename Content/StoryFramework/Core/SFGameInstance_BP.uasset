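; Story Framework game instance that handles save/load after opening a level, camera sensitivity and master volume.
; Delayed events call the save manager to save or load, then push Sensitivity to the player camera manager alongside its existing camera settings.
; Init sets the base sound mix after a short delay.
; SetMasterVolume stores the volume and overrides the Master class in that mix, clamped above zero so silent sounds keep playing.
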(event Custom|LoadAfterOpeningLevel
  (Utilities|FlowControl|Delay 0.2)
  (Default|LoadGame(StoryFramework) (CallFunction|GetSFSaveManager(Controller)))
  (|UpdateCameraSensitivity))

(event Custom|SaveAfterOpeningLevel
  (Utilities|FlowControl|Delay 0.2)
  (Default|SaveGame(StoryFramework) (CallFunction|GetSFSaveManager(Controller)))
  (|UpdateCameraSensitivity))

(event EventInit
  (Utilities|FlowControl|Delay 0.1)
  (Class|GameplayStatics|SetBaseSoundMix "/Game/StoryFramework/Core/Example/Sounds/SFVolume_SCM.SFVolume_SCM"))

(event Custom|SetMasterVolume
  (params (Volume :type Float%20%28double-precision%29))
  (Variables|General|SetMasterVolume Volume)
  (Audio|SetSoundMixClassOverride "/Game/StoryFramework/Core/Example/Sounds/SFVolume_SCM.SFVolume_SCM" "/Engine/EngineSounds/Master.Master" (Math|Float|Clamp(Float) (Variables|General|GetMasterVolume) 0.01) 1.0 0.0 true))