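; Base Blueprint for talkable NPC interactables in StoryFramework, offering a "Talk" prompt labeled with the NPC name from the first dialog set.
; Interacting starts a conversation by passing itself and its DialogSets to NPCManagerAC, which also receives player replies and end-of-conversation requests.
; The construction script sets a single looping-capable animation on the skeletal mesh and offsets the HeadLocation component, while BeginPlay initializes the interaction widget component.
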(event `self.ReceiveBeginPlay`
  ;[0.04314 0.04314 0.05098] Systems (Root)
  (`/Game/StoryFramework/Core/Blueprints/Components/Other/SFInteractionWidget_SC.UpdateInitialization` (`self.SFInteractionWidget_SC`)))

(event `/Game/StoryFramework/Core/Blueprints/BlueprintInterfaces/SFInteraction_BPI.InteractWith`
  (params (DataString :type String))
  ;[0.04314 0.04314 0.05098] Systems (Root)
  (`self.StartConversation`))

(event `InputReply`
  (params (ReplyOption :type Text))
  ;[0.04314 0.04314 0.05098] Systems (Root)
  (`/Game/StoryFramework/Core/Blueprints/Components/Other/NPCManager_AC.InputReply` (`self.NPCManager_AC`) ReplyOption))

(event `InputEndReplies`
  ;[0.04314 0.04314 0.05098] Systems (Root)
  (`/Game/StoryFramework/Core/Blueprints/Components/Other/NPCManager_AC.StopConversation` (`self.NPCManager_AC`) false))

(fn `GetInteractionData`
  (returns (InteractionData :type "/Game/StoryFramework/Core/Blueprints/Structures/InteractableData_S Structure"))
  (bind _values (`BlueprintMapLibrary.Map_Values` (`self.DialogSets`)))
  (return (make `/Game/StoryFramework/Core/Blueprints/Structures/InteractableData_S` (`KismetTextLibrary.Conv_TextToString` (`.NPCName_2_57BB661044410FBA619D0A81E9737FED` (break `/Game/StoryFramework/Core/Blueprints/Structures/NPCInteraction_S` (`|GetArrayItem` _values)))) null null (`self.InteractionPromptOffset`) (`self.DisplayPromptFromRange`) (make `/Game/StoryFramework/Core/Blueprints/Structures/InteractionMethods_S` "NewEnumerator0" "NewEnumerator0" "Talk" null) (struct) (struct) (struct :`InspectMethod` "NewEnumerator0" :`InspectActorOffset` (0.0 0.0 0.0)))))

(fn `StartConversation`
  (`/Game/StoryFramework/Core/Blueprints/Components/Other/NPCManager_AC.InitializeConversation` (`self.NPCManager_AC`) self (`self.DialogSets`)))

(fn `UserConstructionScript`
  (set `SkeletalMeshComponent.AnimationData` (make `SingleAnimationPlayData` (`self.AnimToPlay`)) (`self.SkeletalMesh`))
  (`SceneComponent.K2_AddRelativeLocation` (`self.HeadLocation`) (`self.HeadLocationOffset`) false false))