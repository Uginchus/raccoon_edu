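; Blueprint function library of global gameplay helpers for the Story Framework, covering managers, saving, input, camera, pause UI and dialog movement checks.
; Getters resolve manager components and camera data through messages to player 0's controller and camera manager.
; Save helpers record destroyed, spawned and interacted actors on the SaveManager.
; Others toggle custom-depth outlines, hide first-person components, and swap Enhanced Input contexts, restoring the InteractionManager's cached context on unpause.
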(fn `DestroyActor (SaveGame)`
  (params (Target :type "Actor Object Reference"))
  (`KismetArrayLibrary.Array_Add` (`/Game/StoryFramework/SaveGame/Blueprints/Components/SFSaveManager_AC.DestroyedActors` (`self.GetSFSaveManager (Controller)` null)) (`KismetSystemLibrary.GetObjectName` Target))
  (`Actor.K2_DestroyActor` Target))

(fn `FindMenuButtonInMap (Widget)`
  (params (NamedWidgetsMap :type "Map of Name to Widget Object Reference") (WidgetNavigationData :type "WidgetNavigationData Structure (by ref)"))
  (returns (CustomButtonRef :type "/Game/StoryFramework/Menus/UserInterface/MenuButton_W Object Reference"))
  (bind (_value _returnvalue) (`BlueprintMapLibrary.Map_Find` NamedWidgetsMap (`.WidgetToFocus` (break `WidgetNavigationData` WidgetNavigationData))))
  (bind (_asmenu_button_w _bsuccess) (cast `/Game/StoryFramework/Menus/UserInterface/MenuButton_W` _value :!pure true))
  (if _returnvalue
    (if _bsuccess
      (`/Engine/EditorBlueprintResources/StandardMacros.IsValid` _asmenu_button_w
        (:`Is Valid`
          (`/Game/StoryFramework/Menus/UserInterface/MenuButton_W.CustomHoverButton` _asmenu_button_w false))
        (:`Is Not Valid`
          _))
      (return _asmenu_button_w))))

(fn `GetPauseMenuWidget (Reference)`
  (returns (MenuWidget :type "/Game/StoryFramework/Menus/UserInterface/PauseMenu_W Object Reference"))
  (bind _foundwidgets (`WidgetBlueprintLibrary.GetAllWidgetsOfClass` null "/Game/StoryFramework/Menus/UserInterface/PauseMenu_W.PauseMenu_W_C"))
  (if (`KismetArrayLibrary.Array_IsNotEmpty` _foundwidgets)
    (return (`|GetArrayItem` _foundwidgets))
    (else
      (return null))))

(fn `GetSFCameraSettings (Camera Manager)`
  (returns (CameraSettings :type "/Game/StoryFramework/Core/Blueprints/Structures/GeneralCameraSettings_S Structure"))
  (bind _camerasettings (message `/Game/StoryFramework/Core/Blueprints/BlueprintInterfaces/SFPlayerCameraManager_BPI.GetSFCameraData` (`GameplayStatics.GetPlayerCameraManager` null)))
  (return _camerasettings))

(fn `GetSFInteractionManager (Controller)`
  (returns (InteractionManager :type "/Game/StoryFramework/Core/Blueprints/Components/Core/SFInteractionManager_AC Object Reference"))
  (bind _interactionmanager (message `/Game/StoryFramework/Core/Blueprints/BlueprintInterfaces/SFPlayerControllerData_BPI.GetSFComponents` (`GameplayStatics.GetPlayerController` null)))
  (return _interactionmanager))

(fn `GetSFInventoryManager (Controller)`
  (returns (InventoryManager :type "/Game/StoryFramework/Core/Blueprints/Components/Core/SFInventoryManager_AC Object Reference"))
  (bind (_interactionmanager _inventorymanager) (message `/Game/StoryFramework/Core/Blueprints/BlueprintInterfaces/SFPlayerControllerData_BPI.GetSFComponents` (`GameplayStatics.GetPlayerController` null)))
  (return _inventorymanager))

(fn `GetSFSaveManager (Controller)`
  (returns (SaveManager :type "/Game/StoryFramework/SaveGame/Blueprints/Components/SFSaveManager_AC Object Reference"))
  (bind (_interactionmanager _inventorymanager _sequencemanager _savemanager) (message `/Game/StoryFramework/Core/Blueprints/BlueprintInterfaces/SFPlayerControllerData_BPI.GetSFComponents` (`GameplayStatics.GetPlayerController` null)))
  (return _savemanager))

(fn `GetSFSequenceManager (Controller)`
  (returns (SequenceManager :type "/Game/StoryFramework/Core/Blueprints/Components/Core/SFSequenceManager_AC Object Reference"))
  (bind (_interactionmanager _inventorymanager _sequencemanager) (message `/Game/StoryFramework/Core/Blueprints/BlueprintInterfaces/SFPlayerControllerData_BPI.GetSFComponents` (`GameplayStatics.GetPlayerController` null)))
  (return _sequencemanager))

(fn `GetSFSoundSettingsDataTable`
  (returns (SFSoundSettings :type "/Game/StoryFramework/Core/Blueprints/Structures/SFSoundSettings_S Structure"))
  (bind _returnvalue (`|GetDataTableRow` "/Game/StoryFramework/Core/Blueprints/DataTables/SFSoundSettings_DT.SFSoundSettings_DT" "Editable") ; Play sound from "SFSoundSettings" Data Table.
    (:`then`
      (return _returnvalue))))

(fn `LoadSFComponents (IntoMemory)`
  (`/Game/StoryFramework/Core/Blueprints/Components/Core/SFInteractionManager_AC.LoadSelf` (`self.GetSFInteractionManager (Controller)` null))
  (`/Game/StoryFramework/Core/Blueprints/Components/Core/SFInventoryManager_AC.LoadSelf` (`self.GetSFInventoryManager (Controller)` null)))

(fn `LoadSystemInfo (SaveGame)`
  (returns (SystemData :type "/Game/StoryFramework/SaveGame/Blueprints/Structures/SystemSaveData_S Structure"))
  (bind _returnvalue (`GameplayStatics.LoadGameFromSlot` "SFSaveSlot"))
  (bind _assfsave_game_bp (cast `/Game/StoryFramework/SaveGame/SFSaveGame_BP` _returnvalue))
  (return (`/Game/StoryFramework/SaveGame/SFSaveGame_BP.SystemData` _assfsave_game_bp)))

(fn `OutlineActor (PostProcess)`
  (params (Actor :type "Actor Object Reference") (Remove :type Boolean))
  (bind _returnvalue (`Actor.K2_GetComponentsByClass` Actor "/Script/Engine.SkeletalMeshComponent"))
  (bind _returnvalue_2 (`Actor.K2_GetComponentsByClass` Actor "/Script/Engine.StaticMeshComponent"))
  (bind _returnvalue_3 (not Remove))
  (`/Engine/EditorBlueprintResources/StandardMacros.IsValid` Actor
    (:`Is Valid`
      (if (>= (`KismetArrayLibrary.Array_LastIndex` _returnvalue_2) 0)
        (for _array_element _returnvalue_2
          (`PrimitiveComponent.SetRenderCustomDepth` _array_element _returnvalue_3)))
      (if (>= (`KismetArrayLibrary.Array_LastIndex` _returnvalue) 0)
        (for _array_element_2 _returnvalue
          (`PrimitiveComponent.SetRenderCustomDepth` _array_element_2 _returnvalue_3))))))

(fn `ResetSFCameraStates (Camera Manager)`
  (bind _sfcameramanagerref (message `/Game/StoryFramework/Core/Blueprints/BlueprintInterfaces/SFPlayerCameraManager_BPI.GetSFCameraManager` (`GameplayStatics.GetPlayerCameraManager` null)))
  (`/Game/StoryFramework/Core/Blueprints/SFPlayerCamera_PCM.ResetStates` _sfcameramanagerref))

(fn `SaveSpawnedActor (SaveGame)`
  (params (Target :type "Actor Object Reference (by ref)") (`Interactable Data` :type "/Game/StoryFramework/Core/Blueprints/Structures/InteractableData_S Structure") (StaticMeshActor :type "StaticMesh Object Reference"))
  (`KismetArrayLibrary.Array_Add` (`/Game/StoryFramework/SaveGame/Blueprints/Components/SFSaveManager_AC.SpawnedActors` (`self.GetSFSaveManager (Controller)` null)) (make `/Game/StoryFramework/SaveGame/Blueprints/Structures/LevelActorSaveData_S` (`GameplayStatics.GetObjectClass` Target) (`Actor.GetTransform` Target) (`Actor.Tags` Target) `Interactable Data` StaticMeshActor)))

(fn `SFMovementCondition (Dialog Manager)`
  (returns (ReturnValue :type Boolean))
  (bind _interactionmanager (`self.GetSFInteractionManager (Controller)` null))
  (if (and (`/Game/StoryFramework/Core/Blueprints/Components/Core/SFInteractionManager_AC.IsInDialogWithNPC` _interactionmanager) (`KismetSystemLibrary.IsValid` (`/Game/StoryFramework/Core/Blueprints/Components/Core/SFInteractionManager_AC.TargetNPCActor` _interactionmanager)))
    (return (`.AllowPlayerMovement_14_3F0FDE4443D6842A238E39B6BCEC142B` (break `/Game/StoryFramework/Core/Blueprints/Structures/NPCInteraction_S` (`/Game/StoryFramework/Core/Blueprints/Components/Other/NPCManager_AC.CurrentDialogSet` (`/Game/StoryFramework/Core/Blueprints/NPCInteractableBase_BP.NPCManager_AC` (`/Game/StoryFramework/Core/Blueprints/Components/Core/SFInteractionManager_AC.TargetNPCActor` _interactionmanager))))))
    (else
      (return true))))

(fn `SimpleFirstPersonComponentHide`
  (params (Target :type "SceneComponent Object Reference"))
  (bind (_camerasettings _camerarelativeoffset _iscameralookinputlocked _currentcamerapreset) (message `/Game/StoryFramework/Core/Blueprints/BlueprintInterfaces/SFPlayerCameraManager_BPI.GetSFCameraData` (`GameplayStatics.GetPlayerCameraManager` null)))
  (`SceneComponent.SetVisibility` Target (select `bool` (`/Game/StoryFramework/Core/Blueprints/Components/Core/SFSequenceManager_AC.IsCurrentSequencePlaying` (`self.GetSFSequenceManager (Controller)` null)) :`false` (select `/Game/StoryFramework/Core/Blueprints/Enumerators/CameraPresets_E` _currentcamerapreset :`NewEnumerator3` true :`NewEnumerator7` true) :`true` true) false))

(fn `TogglePauseGame (Widget)`
  (params (PauseWidgetClass :type "UserWidget Class Reference") (UseWidgetNavInputMapping :type Boolean))
  (locals (TargetMappingContext :type "InputMappingContext Object Reference") (NewLocalVar :type "InputMappingContext Object Reference") (TargetUseWidgetNav :type Boolean))
  (bind _returnvalue (`GameplayStatics.GetPlayerController` null))
  (bind _returnvalue_2 (`GameplayStatics.GetPlayerController` null))
  (bind _targetusewidgetnav (`local.TargetUseWidgetNav`))
  (set `local.TargetUseWidgetNav` UseWidgetNavInputMapping)
  (bind _foundwidgets (`WidgetBlueprintLibrary.GetAllWidgetsOfClass` null PauseWidgetClass))
  (bind _output (`|GetArrayItem` _foundwidgets))
  (`/Engine/EditorBlueprintResources/StandardMacros.IsValid` _output
    (:`Is Valid`
      (`Widget.RemoveFromParent` _output)
      (`GameplayStatics.SetGamePaused` null)
      (set `PlayerController.bShowMouseCursor` false _returnvalue_2)
      (`WidgetBlueprintLibrary.SetInputMode_GameOnly` _returnvalue_2 true)
      (if _targetusewidgetnav
        (`self.UpdateInputMappingContext` (`/Game/StoryFramework/Core/Blueprints/Components/Core/SFInteractionManager_AC.CurrentInputMappingContext` (`self.GetSFInteractionManager (Controller)` null)))))
    (:`Is Not Valid`
      (bind _returnvalue_3 (`|CreateWidget` PauseWidgetClass))
      (`UserWidget.AddToViewport` _returnvalue_3 0)
      (`GameplayStatics.SetGamePaused` null true)
      (set `PlayerController.bShowMouseCursor` true _returnvalue)
      (`WidgetBlueprintLibrary.SetInputMode_GameAndUIEx` _returnvalue _returnvalue_3 "DoNotLock" false true)
      (if _targetusewidgetnav
        (`self.UpdateInputMappingContext` "/Game/StoryFramework/Menus/Input/WidgetMenu_IMC.WidgetMenu_IMC" false)))))

(fn `UpdateInputMappingContext`
  (params (NewMappingContext :type "InputMappingContext Object Reference") (UpdateInteractionVariable :type Boolean :default true))
  (bind _interactionmanager (`self.GetSFInteractionManager (Controller)` null))
  (bind _returnvalue (pcsubsystem `EnhancedInputLocalPlayerSubsystem` (`GameplayStatics.GetPlayerController` null)))
  (`EnhancedInputSubsystemInterface.ClearAllMappings` _returnvalue)
  (`EnhancedInputSubsystemInterface.AddMappingContext` _returnvalue NewMappingContext 0 (make `ModifyContextOptions` true))
  (if UpdateInteractionVariable
    (`/Engine/EditorBlueprintResources/StandardMacros.IsValid` _interactionmanager
      (:`Is Valid`
        (set `/Game/StoryFramework/Core/Blueprints/Components/Core/SFInteractionManager_AC.CurrentInputMappingContext` NewMappingContext _interactionmanager)))))

(fn `UpdateInteractActors (SaveGame)`
  (params (InteractActor :type "/Game/StoryFramework/Core/Blueprints/InteractableBase_BP Object Reference") (DataString :type String))
  (locals (FindInteractActorNames :type "Array of String") (TargetInteractActor :type "/Game/StoryFramework/Core/Blueprints/InteractableBase_BP Object Reference") (TargetInteractDataString :type String))
  (bind _savemanager (`self.GetSFSaveManager (Controller)` null))
  (set `local.TargetInteractActor` InteractActor)
  (set `local.TargetInteractDataString` DataString)
  (bind _keys (`BlueprintMapLibrary.Map_Keys` (`/Game/StoryFramework/SaveGame/Blueprints/Components/SFSaveManager_AC.InteractActors` _savemanager)))
  (for _array_element _keys
    (`KismetArrayLibrary.Array_Add` (`local.FindInteractActorNames`) _array_element))
  (`BlueprintMapLibrary.Map_Add` (`/Game/StoryFramework/SaveGame/Blueprints/Components/SFSaveManager_AC.InteractActors` _savemanager) (`KismetSystemLibrary.GetObjectName` (`local.TargetInteractActor`)) (`local.TargetInteractDataString`)))