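; General-purpose Blueprint function library for StoryFramework, offering stateless math, transform, debug and trace helpers.
; It covers range mapping, random values, vector easing, array sums, input direction, look-at rotations and by-ref transform component setters.
; Typed print wrappers format values and share a PrintSettings struct.
; Bounce line traces by channel, object type or profile chain hits by mirroring each trace off the impact normal, stopping when a hit is not blocking.
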(fn `BounceLineTraceByChannel`
  (params (Start :type "Vector Structure") (End :type "Vector Structure") (Bounces :type Integer) (BounceReach :type "Float (double-precision)") (TraceChannel :type "ETraceTypeQuery Enum" :default "TraceTypeQuery1") (TraceComplex :type Boolean) (DrawDebugType :type "EDrawDebugTrace Enum" :default "None"))
  (returns (OutHits :type "Array of HitResult Structure"))
  (locals (PreviousHitResult :type "HitResult Structure") (TraceDistance :type "Float (double-precision)" :default 5000.0) (OutHitResults :type "Array of HitResult Structure"))
  (bind (_bblockinghit _binitialoverlap _time _distance _location _impactpoint _normal _impactnormal _physmat _hitactor _hitcomponent _hitbonename _bonename _hititem _elementindex _faceindex _tracestart _traceend) (`GameplayStatics.BreakHitResult` (`local.PreviousHitResult`)))
  (bind _returnvalue (`KismetMathLibrary.Normal` (`KismetMathLibrary.MirrorVectorByNormal` (- _traceend _tracestart) _impactnormal)))
  (bind _outhit (`KismetSystemLibrary.LineTraceSingle` :`Start` Start :`End` End :`TraceChannel` TraceChannel :`bTraceComplex` TraceComplex :`DrawDebugType` DrawDebugType))
  (bind _output_get (set `local.PreviousHitResult` _outhit))
  (`KismetArrayLibrary.Array_Add` (`local.OutHitResults`) _output_get)
  (for _ (range 1 (+ Bounces 1))
    (if _bblockinghit
      (bind _outhit_2 (`KismetSystemLibrary.LineTraceSingle` :`Start` (+ _impactpoint _returnvalue) :`End` (+ (* _returnvalue BounceReach) _impactpoint) :`TraceChannel` TraceChannel :`bTraceComplex` TraceComplex :`DrawDebugType` DrawDebugType))
      (bind _output_get_2 (set `local.PreviousHitResult` _outhit_2))
      (`KismetArrayLibrary.Array_Add` (`local.OutHitResults`) _output_get_2)
      (else
        (break))))
  (return (`local.OutHitResults`)))

(fn `BounceLineTraceByProfile`
  (params (Start :type "Vector Structure") (End :type "Vector Structure") (Bounces :type Integer) (BounceReach :type "Float (double-precision)") (ProfileName :type Name) (TraceComplex :type Boolean) (DrawDebugType :type "EDrawDebugTrace Enum" :default "None"))
  (returns (OutHits :type "Array of HitResult Structure"))
  (locals (PreviousHitResult :type "HitResult Structure") (TraceDistance :type "Float (double-precision)" :default 5000.0) (OutHitResults :type "Array of HitResult Structure"))
  (bind (_bblockinghit _binitialoverlap _time _distance _location _impactpoint _normal _impactnormal _physmat _hitactor _hitcomponent _hitbonename _bonename _hititem _elementindex _faceindex _tracestart _traceend) (`GameplayStatics.BreakHitResult` (`local.PreviousHitResult`)))
  (bind _returnvalue (`KismetMathLibrary.Normal` (`KismetMathLibrary.MirrorVectorByNormal` (- _traceend _tracestart) _impactnormal)))
  (bind _outhit (`KismetSystemLibrary.LineTraceSingleByProfile` :`Start` Start :`End` End :`ProfileName` ProfileName :`bTraceComplex` TraceComplex :`DrawDebugType` DrawDebugType))
  (bind _output_get (set `local.PreviousHitResult` _outhit))
  (`KismetArrayLibrary.Array_Add` (`local.OutHitResults`) _output_get)
  (for _ (range 1 (+ Bounces 1))
    (if _bblockinghit
      (bind _outhit_2 (`KismetSystemLibrary.LineTraceSingleByProfile` :`Start` (+ _impactpoint _returnvalue) :`End` (+ (* _returnvalue BounceReach) _impactpoint) :`ProfileName` ProfileName :`bTraceComplex` TraceComplex :`DrawDebugType` DrawDebugType))
      (bind _output_get_2 (set `local.PreviousHitResult` _outhit_2))
      (`KismetArrayLibrary.Array_Add` (`local.OutHitResults`) _output_get_2)
      (else
        (break))))
  (return (`local.OutHitResults`)))

(fn `BounceLineTraceForObjects`
  (params (Start :type "Vector Structure") (End :type "Vector Structure") (Bounces :type Integer) (BounceReach :type "Float (double-precision)") (ObjectTypes :type "Array of EObjectTypeQuery Enum (by ref)") (TraceComplex :type Boolean) (DrawDebugType :type "EDrawDebugTrace Enum" :default "None"))
  (returns (OutHits :type "Array of HitResult Structure"))
  (locals (PreviousHitResult :type "HitResult Structure") (TraceDistance :type "Float (double-precision)" :default 5000.0) (OutHitResults :type "Array of HitResult Structure"))
  (bind (_bblockinghit _binitialoverlap _time _distance _location _impactpoint _normal _impactnormal _physmat _hitactor _hitcomponent _hitbonename _bonename _hititem _elementindex _faceindex _tracestart _traceend) (`GameplayStatics.BreakHitResult` (`local.PreviousHitResult`)))
  (bind _returnvalue (`KismetMathLibrary.Normal` (`KismetMathLibrary.MirrorVectorByNormal` (- _traceend _tracestart) _impactnormal)))
  (bind _outhit (`KismetSystemLibrary.LineTraceSingleForObjects` :`Start` Start :`End` End :`ObjectTypes` ObjectTypes :`bTraceComplex` TraceComplex :`DrawDebugType` DrawDebugType))
  (bind _output_get (set `local.PreviousHitResult` _outhit))
  (`KismetArrayLibrary.Array_Add` (`local.OutHitResults`) _output_get)
  (for _ (range 1 (+ Bounces 1))
    (if _bblockinghit
      (bind _outhit_2 (`KismetSystemLibrary.LineTraceSingleForObjects` :`Start` (+ _impactpoint _returnvalue) :`End` (+ (* _returnvalue BounceReach) _impactpoint) :`ObjectTypes` ObjectTypes :`bTraceComplex` TraceComplex :`DrawDebugType` DrawDebugType))
      (bind _output_get_2 (set `local.PreviousHitResult` _outhit_2))
      (`KismetArrayLibrary.Array_Add` (`local.OutHitResults`) _output_get_2)
      (else
        (break))))
  (return (`local.OutHitResults`)))

(fn `FindActorLookAtRotation`
  (params (Start :type "Actor Object Reference") (End :type "Actor Object Reference"))
  (returns (ReturnValue :type "Rotator Structure"))
  (return (`KismetMathLibrary.FindLookAtRotation` (`Actor.K2_GetActorLocation` Start) (`Actor.K2_GetActorLocation` End))))

(fn `FindActorLookAtRotationFromLocation`
  (params (Start :type "Actor Object Reference") (End :type "Vector Structure"))
  (returns (ReturnValue :type "Rotator Structure"))
  (return (`KismetMathLibrary.FindLookAtRotation` (`Actor.K2_GetActorLocation` Start) End)))

(fn `GetDistanceBetweenVectors`
  (params (A :type "Vector Structure") (B :type "Vector Structure"))
  (returns (ReturnValue :type "Float (double-precision)"))
  (return (`KismetMathLibrary.VSize` (- A B))))

(fn `GetFloatAsPercentage`
  (params (Value :type "Float (double-precision)") (`Value Min` :type "Float (double-precision)") (`Value Max` :type "Float (double-precision)"))
  (returns (`Output Value` :type "Float (double-precision)"))
  (return (`KismetMathLibrary.MapRangeClamped` Value `Value Min` `Value Max` 0.0 100.0)))

(fn `GetInputDirection`
  (params (ControlRotation :type "Rotator Structure") (ForwardAxisValue :type "Float (double-precision)") (RightAxisValue :type "Float (double-precision)"))
  (returns (Yaw :type "Float (double-precision)") (Pitch :type "Float (double-precision)"))
  (bind (_yaw _pitch) (`KismetMathLibrary.GetYawPitchFromVector` (+ (* (`KismetMathLibrary.GetForwardVector` ControlRotation) ForwardAxisValue) (* (`KismetMathLibrary.GetRightVector` ControlRotation) RightAxisValue))))
  (return _yaw _pitch))

(fn `GetIntegerAsPercentage`
  (params (Value :type Integer) (`Value Min` :type Integer) (`Value Max` :type Integer))
  (returns (`Output Value` :type Integer))
  (return (`self.IntegerMapRangedClamped` Value `Value Min` `Value Max` 0 100)))

(fn `GetTranformLocation`
  (params (Tranform :type "Transform Structure"))
  (returns (ReturnValue :type "Vector Structure"))
  (return (.location Tranform)))

(fn `GetTranformRotation`
  (params (Tranform :type "Transform Structure"))
  (returns (ReturnValue :type "Rotator Structure"))
  (return (.rotation Tranform)))

(fn `GetTranformScale`
  (params (Tranform :type "Transform Structure"))
  (returns (ReturnValue :type "Vector Structure"))
  (return (.scale Tranform)))

(fn `GetVector2DValueAsDirection`
  (params (Vector2D :type "Vector2D Structure"))
  (returns (Direction :type String))
  (locals (TargetVector2D :type "Vector2D Structure"))
  (set `local.TargetVector2D` Vector2D)
  (return (`KismetMathLibrary.SelectString` "Right" (`KismetMathLibrary.SelectString` "Left" (`KismetMathLibrary.SelectString` "Down" "Up" (`KismetMathLibrary.EqualExactly_Vector2DVector2D` (`local.TargetVector2D`) (0.0 1.0))) (`KismetMathLibrary.EqualExactly_Vector2DVector2D` (`local.TargetVector2D`) (-1.0 0.0))) (`KismetMathLibrary.EqualExactly_Vector2DVector2D` (`local.TargetVector2D`) (1.0 0.0)))))

(fn `GetVectorDistancedFromOrigin`
  (params (Origin :type "Vector Structure") (Direction :type "Vector Structure") (Distance :type "Float (double-precision)"))
  (returns (Start :type "Vector Structure") (End :type "Vector Structure"))
  (return Origin (+ Origin (* Direction Distance))))

(fn `IntegerMapRangedClamped`
  (params (Value :type Integer) (`In Range A` :type Integer) (`In Range B` :type Integer) (`Out Range A` :type Integer) (`Out Range B` :type Integer))
  (returns (`Output Value` :type Integer))
  (return (`KismetMathLibrary.FTrunc` (`KismetMathLibrary.MapRangeClamped` (`KismetMathLibrary.Conv_IntToDouble` `In Range A`) (`KismetMathLibrary.Conv_IntToDouble` Value) (`KismetMathLibrary.Conv_IntToDouble` `Out Range B`) (`KismetMathLibrary.Conv_IntToDouble` `Out Range A`) (`KismetMathLibrary.Conv_IntToDouble` `In Range B`)))))

(fn `IntegerMapRangedUnclamped`
  (params (Value :type Integer) (`In Range A` :type Integer) (`In Range B` :type Integer) (`Out Range A` :type Integer) (`Out Range B` :type Integer))
  (returns (`Output Value` :type Integer))
  (return (`KismetMathLibrary.FTrunc` (`KismetMathLibrary.MapRangeUnclamped` (`KismetMathLibrary.Conv_IntToDouble` Value) (`KismetMathLibrary.Conv_IntToDouble` `In Range A`) (`KismetMathLibrary.Conv_IntToDouble` `In Range B`) (`KismetMathLibrary.Conv_IntToDouble` `Out Range A`) (`KismetMathLibrary.Conv_IntToDouble` `Out Range B`)))))

(fn `PrintBool`
  (params (InBool :type Boolean) (Key :type Name) (PrintSettings :type "/Game/StoryFramework/Core/Blueprints/Structures/PrintDebugSettings_S Structure"))
  (bind (_printtoscreen _printtolog _textcolor _duration) (break `/Game/StoryFramework/Core/Blueprints/Structures/PrintDebugSettings_S` PrintSettings))
  (`KismetSystemLibrary.PrintString` null (`KismetStringLibrary.Conv_BoolToString` InBool) _printtoscreen _printtolog _textcolor _duration Key))

(fn `PrintFloat`
  (params (InFloat :type "Float (double-precision)") (RoundFloat :type Boolean) (Key :type Name) (PrintSettings :type "/Game/StoryFramework/Core/Blueprints/Structures/PrintDebugSettings_S Structure"))
  (bind (_printtoscreen _printtolog _textcolor _duration) (break `/Game/StoryFramework/Core/Blueprints/Structures/PrintDebugSettings_S` PrintSettings))
  (`KismetSystemLibrary.PrintString` null (`KismetMathLibrary.SelectString` (`KismetStringLibrary.Conv_IntToString` (`KismetMathLibrary.Round` InFloat)) (`KismetStringLibrary.Conv_DoubleToString` InFloat) RoundFloat) _printtoscreen _printtolog _textcolor _duration Key))

(fn `PrintInt`
  (params (InInt :type Integer) (Key :type Name) (PrintSettings :type "/Game/StoryFramework/Core/Blueprints/Structures/PrintDebugSettings_S Structure"))
  (bind (_printtoscreen _printtolog _textcolor _duration) (break `/Game/StoryFramework/Core/Blueprints/Structures/PrintDebugSettings_S` PrintSettings))
  (`KismetSystemLibrary.PrintString` null (`KismetStringLibrary.Conv_IntToString` InInt) _printtoscreen _printtolog _textcolor _duration Key))

(fn `PrintRotator`
  (params (InRot :type "Rotator Structure") (`X(Roll)` :type Boolean :default true) (`Y(Pitch)` :type Boolean :default true) (`Z(Yaw)` :type Boolean :default true) (Key :type Name) (PrintSettings :type "/Game/StoryFramework/Core/Blueprints/Structures/PrintDebugSettings_S Structure"))
  (bind (_printtoscreen _printtolog _textcolor _duration) (break `/Game/StoryFramework/Core/Blueprints/Structures/PrintDebugSettings_S` PrintSettings))
  (`KismetSystemLibrary.PrintString` null (`KismetStringLibrary.Concat_StrStr` (`KismetMathLibrary.SelectString` (`KismetStringLibrary.Concat_StrStr` "X(Roll)=" (`KismetStringLibrary.Conv_DoubleToString` (.roll InRot)) " ") "" `X(Roll)`) (`KismetMathLibrary.SelectString` (`KismetStringLibrary.Concat_StrStr` "Y(Pitch)=" (`KismetStringLibrary.Conv_DoubleToString` (.pitch InRot)) " ") "" `Y(Pitch)`) (`KismetMathLibrary.SelectString` (`KismetStringLibrary.Concat_StrStr` "Z(Yaw)=" (`KismetStringLibrary.Conv_DoubleToString` (.yaw InRot)) " ") "" `Z(Yaw)`)) _printtoscreen _printtolog _textcolor _duration Key))

(fn `PrintStringArray`
  (params (InStrings :type "Array of String") (Key :type Name) (PrintSettings :type "/Game/StoryFramework/Core/Blueprints/Structures/PrintDebugSettings_S Structure"))
  (locals (AppendedString :type String))
  (bind (_printtoscreen _printtolog _textcolor _duration) (break `/Game/StoryFramework/Core/Blueprints/Structures/PrintDebugSettings_S` PrintSettings))
  (bind _appendedstring (`local.AppendedString`))
  (for _array_element InStrings
    (set `local.AppendedString` (`KismetStringLibrary.Concat_StrStr` _appendedstring _array_element)))
  (`KismetSystemLibrary.PrintString` null _appendedstring _printtoscreen _printtolog _textcolor _duration Key))

(fn `PrintTransform`
  (params (InTransform :type "Transform Structure") (Key :type Name) (PrintSettings :type "/Game/StoryFramework/Core/Blueprints/Structures/PrintDebugSettings_S Structure"))
  (bind (_printtoscreen _printtolog _textcolor _duration) (break `/Game/StoryFramework/Core/Blueprints/Structures/PrintDebugSettings_S` PrintSettings))
  (for _index (range 3)
    (`KismetSystemLibrary.PrintString` null (select `int` _index :`0` (`KismetStringLibrary.Concat_StrStr` "Scale: " (`KismetStringLibrary.Conv_VectorToString` (.scale InTransform))) :`1` (`KismetStringLibrary.Concat_StrStr` "Rotation: " (`KismetStringLibrary.Conv_RotatorToString` (.rotation InTransform))) :`2` (`KismetStringLibrary.Concat_StrStr` "Location: " (`KismetStringLibrary.Conv_VectorToString` (.location InTransform)))) _printtoscreen _printtolog _textcolor _duration Key)))

(fn `PrintVector`
  (params (InVec :type "Vector Structure") (X :type Boolean :default true) (Y :type Boolean :default true) (Z :type Boolean :default true) (Key :type Name) (PrintSettings :type "/Game/StoryFramework/Core/Blueprints/Structures/PrintDebugSettings_S Structure"))
  (bind (_printtoscreen _printtolog _textcolor _duration) (break `/Game/StoryFramework/Core/Blueprints/Structures/PrintDebugSettings_S` PrintSettings))
  (`KismetSystemLibrary.PrintString` null (`KismetStringLibrary.Concat_StrStr` (`KismetMathLibrary.SelectString` (`KismetStringLibrary.Concat_StrStr` "X=" (`KismetStringLibrary.Conv_DoubleToString` (.x InVec)) " ") "" X) (`KismetMathLibrary.SelectString` (`KismetStringLibrary.Concat_StrStr` "Y=" (`KismetStringLibrary.Conv_DoubleToString` (.y InVec)) " ") "" Y) (`KismetMathLibrary.SelectString` (`KismetStringLibrary.Concat_StrStr` "Z=" (`KismetStringLibrary.Conv_DoubleToString` (.z InVec)) " ") "" Z)) _printtoscreen _printtolog _textcolor _duration Key))

(fn `RandomColor`
  (params (`Randomize Color Alpha` :type Boolean))
  (returns (`Output Value` :type "SlateColor Structure"))
  (return (make `SlateColor` (select `bool` `Randomize Color Alpha` :`false` (make `LinearColor` (`KismetMathLibrary.RandomFloat`) (`KismetMathLibrary.RandomFloat`) (`KismetMathLibrary.RandomFloat`) 1.0) :`true` (make `LinearColor` (`KismetMathLibrary.RandomFloat`) (`KismetMathLibrary.RandomFloat`) (`KismetMathLibrary.RandomFloat`) (`KismetMathLibrary.RandomFloat`))))))

(fn `RandomVectorInRange`
  (params (UniformScale :type Boolean) (`Min Scale` :type "Float (double-precision)") (`Max Scale` :type "Float (double-precision)"))
  (returns (`Output Value` :type "Vector Structure"))
  (bind _returnvalue (`KismetMathLibrary.RandomFloatInRange` `Min Scale` `Max Scale`))
  (return (select `bool` UniformScale :`false` (`KismetMathLibrary.MakeVector` (`KismetMathLibrary.RandomFloatInRange` `Min Scale` `Max Scale`) (`KismetMathLibrary.RandomFloatInRange` `Min Scale` `Max Scale`) (`KismetMathLibrary.RandomFloatInRange` `Min Scale` `Max Scale`)) :`true` (`KismetMathLibrary.MakeVector` _returnvalue _returnvalue _returnvalue))))

(fn `SetTranformLoc (ByRef)`
  (params (Tranform :type "Transform Structure (by ref)") (InLoc :type "Vector Structure"))
  (`|VariableSetRef` Tranform (`KismetMathLibrary.MakeTransform` InLoc (.rotation Tranform) (.scale Tranform))))

(fn `SetTransformRot (ByRef)`
  (params (Tranform :type "Transform Structure (by ref)") (InRot :type "Rotator Structure"))
  (`|VariableSetRef` Tranform (`KismetMathLibrary.MakeTransform` (.location Tranform) InRot (.scale Tranform))))

(fn `SetTransformScale (ByRef)`
  (params (Tranform :type "Transform Structure (by ref)") (Scale :type "Vector Structure"))
  (`|VariableSetRef` Tranform (`KismetMathLibrary.MakeTransform` (.location Tranform) (.rotation Tranform) Scale)))

(fn `SumArray (Float)`
  (params (`Float Array` :type "Array of Float (double-precision)"))
  (returns (ReturnValue :type "Float (double-precision)"))
  (locals (SumOfArray :type "Float (double-precision)"))
  (for _array_element `Float Array`
    (set `local.SumOfArray` (+ _array_element (`local.SumOfArray`))))
  (return (`local.SumOfArray`)))

(fn `SumArray (Vector)`
  (params (VectorArray :type "Array of Vector Structure"))
  (returns (ReturnValue :type "Vector Structure"))
  (locals (SumOfArray :type "Vector Structure"))
  (for _array_element VectorArray
    (set `local.SumOfArray` (+ _array_element (`local.SumOfArray`))))
  (return (`local.SumOfArray`)))

(fn `VInterpEaseInOut`
  (params (A :type "Vector Structure") (B :type "Vector Structure") (Alpha :type "Float (double-precision)") (Exponent :type "Float (double-precision)"))
  (returns (ReturnValue :type "Vector Structure"))
  (return (`KismetMathLibrary.MakeVector` (`KismetMathLibrary.FInterpEaseInOut` (.x A) (.x B) Alpha Exponent) (`KismetMathLibrary.FInterpEaseInOut` (.y A) (.y B) Alpha Exponent) (`KismetMathLibrary.FInterpEaseInOut` (.z A) (.z B) Alpha Exponent))))