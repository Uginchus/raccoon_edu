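; BP_Candle_04 is a candle prop with a point light that can be switched on or off.
; The construction script reads LightOn to either apply the configured intensity and attenuation radius and show Plane1, or zero the intensity and hide that plane.
; It has no runtime logic, as the event graph holds only empty events.
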(event `self.ReceiveBeginPlay`)

(fn `UserConstructionScript`
  (if (`self.Light On`)
    (`LightComponent.SetIntensity` (`self.PointLight`) (`self.LightIntensity`))
    (`LocalLightComponent.SetAttenuationRadius` (`self.PointLight`) (`self.AttenuationRadius`))
    (`SceneComponent.SetVisibility` (`self.Plane1`) true false)
    (else
      (`LightComponent.SetIntensity` (`self.PointLight`) 0.0)
      (`SceneComponent.SetVisibility` (`self.Plane1`) false false))))